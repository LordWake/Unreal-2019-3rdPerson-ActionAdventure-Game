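; BP_MenuUI is a menu UI Blueprint that passes gamepad face button presses to the menu canvas.
; Each press event casts the Canvas reference to BP_MenuCanvas and sets the matching Y, A, X or B button flag to true.
; It only raises these flags, with no release handling, reset or menu logic of its own.
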(event `Key|Gamepad_FaceButton_Top`
  (params (Key :type "Key Structure"))
  (:`Pressed`
    (bind _asbp_menu_canvas (cast `/Game/Blueprints/Managers/BP_MenuCanvas` (`self.canvas`)))
    (set `/Game/Blueprints/Managers/BP_MenuCanvas.YButton` true _asbp_menu_canvas)))

(event `Key|Gamepad_FaceButton_Bottom`
  (params (Key :type "Key Structure"))
  (:`Pressed`
    (bind _asbp_menu_canvas (cast `/Game/Blueprints/Managers/BP_MenuCanvas` (`self.canvas`)))
    (set `/Game/Blueprints/Managers/BP_MenuCanvas.AButton` true _asbp_menu_canvas)))

(event `Key|Gamepad_FaceButton_Left`
  (params (Key :type "Key Structure"))
  (:`Pressed`
    (bind _asbp_menu_canvas (cast `/Game/Blueprints/Managers/BP_MenuCanvas` (`self.canvas`)))
    (set `/Game/Blueprints/Managers/BP_MenuCanvas.XButton` true _asbp_menu_canvas)))

(event `Key|Gamepad_FaceButton_Right`
  (params (Key :type "Key Structure"))
  (:`Pressed`
    (bind _asbp_menu_canvas (cast `/Game/Blueprints/Managers/BP_MenuCanvas` (`self.canvas`)))
    (set `/Game/Blueprints/Managers/BP_MenuCanvas.BButton` true _asbp_menu_canvas)))

(fn `UserConstructionScript`)