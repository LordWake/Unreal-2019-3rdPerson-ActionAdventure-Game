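; BP_MagicEnemySpawner is a one-shot trigger that spawns a magic enemy and seals two magic block walls when the player character enters its box.
; On BeginPlay it opens BlockWall and BlockWallTwo by ignoring all collision channels and deactivating their three effects.
; Player overlap calls SpawnMagicEnemy, restores blocking collision and effects on both walls, then destroys the spawner.
; Nothing in this graph reopens the walls.
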(event `self.ReceiveBeginPlay`
  (`|ExecutionSequence`
    (:`then_0`
      (bind _asbp_magic_block (cast `/Game/Blueprints/Enemies/BP_MagicBlock` (`self.blockWall`)))
      (`|ExecutionSequence`
        (:`then_0`
          (`PrimitiveComponent.SetCollisionResponseToAllChannels` (`/Game/Blueprints/Enemies/BP_MagicBlock.BoxCollision` _asbp_magic_block) "ECR_Ignore"))
        (:`then_1`
          (`ActorComponent.Deactivate` (`/Game/Blueprints/Enemies/BP_MagicBlock.FX1` _asbp_magic_block)))
        (:`then_2`
          (`ActorComponent.Deactivate` (`/Game/Blueprints/Enemies/BP_MagicBlock.FX2` _asbp_magic_block)))
        (:`then_3`
          (`ActorComponent.Deactivate` (`/Game/Blueprints/Enemies/BP_MagicBlock.FX3` _asbp_magic_block)))))
    (:`then_1`
      (bind _asbp_magic_block_2 (cast `/Game/Blueprints/Enemies/BP_MagicBlock` (`self.blockWallTwo`)))
      (`|ExecutionSequence`
        (:`then_0`
          (`PrimitiveComponent.SetCollisionResponseToAllChannels` (`/Game/Blueprints/Enemies/BP_MagicBlock.BoxCollision` _asbp_magic_block_2) "ECR_Ignore"))
        (:`then_1`
          (`ActorComponent.Deactivate` (`/Game/Blueprints/Enemies/BP_MagicBlock.FX1` _asbp_magic_block_2)))
        (:`then_2`
          (`ActorComponent.Deactivate` (`/Game/Blueprints/Enemies/BP_MagicBlock.FX2` _asbp_magic_block_2)))
        (:`then_3`
          (`ActorComponent.Deactivate` (`/Game/Blueprints/Enemies/BP_MagicBlock.FX3` _asbp_magic_block_2)))))))

(event `self.Box.OnComponentBeginOverlap`
  (params (OverlappedComponent :type "PrimitiveComponent Object Reference") (OtherActor :type "Actor Object Reference") (OtherComp :type "PrimitiveComponent Object Reference") (OtherBodyIndex :type Integer) (bFromSweep :type Boolean) (SweepResult :type "HitResult Structure (by ref)"))
  (cast `/Game/Blueprints/Player/BP_MyCharacter` OtherActor)
  (`self.SpawnMagicEnemy`)
  (`|ExecutionSequence`
    (:`then_0`
      (bind _asbp_magic_block (cast `/Game/Blueprints/Enemies/BP_MagicBlock` (`self.blockWall`)))
      (`|ExecutionSequence`
        (:`then_0`
          (`PrimitiveComponent.SetCollisionResponseToAllChannels` (`/Game/Blueprints/Enemies/BP_MagicBlock.BoxCollision` _asbp_magic_block) "ECR_Block"))
        (:`then_1`
          (`ActorComponent.Activate` (`/Game/Blueprints/Enemies/BP_MagicBlock.FX1` _asbp_magic_block) false))
        (:`then_2`
          (`ActorComponent.Activate` (`/Game/Blueprints/Enemies/BP_MagicBlock.FX2` _asbp_magic_block) false))
        (:`then_3`
          (`ActorComponent.Activate` (`/Game/Blueprints/Enemies/BP_MagicBlock.FX3` _asbp_magic_block) false))))
    (:`then_1`
      (bind _asbp_magic_block_2 (cast `/Game/Blueprints/Enemies/BP_MagicBlock` (`self.blockWallTwo`)))
      (`|ExecutionSequence`
        (:`then_0`
          (`PrimitiveComponent.SetCollisionResponseToAllChannels` (`/Game/Blueprints/Enemies/BP_MagicBlock.BoxCollision` _asbp_magic_block_2) "ECR_Block"))
        (:`then_1`
          (`ActorComponent.Activate` (`/Game/Blueprints/Enemies/BP_MagicBlock.FX1` _asbp_magic_block_2) false))
        (:`then_2`
          (`ActorComponent.Activate` (`/Game/Blueprints/Enemies/BP_MagicBlock.FX2` _asbp_magic_block_2) false))
        (:`then_3`
          (`ActorComponent.Activate` (`/Game/Blueprints/Enemies/BP_MagicBlock.FX3` _asbp_magic_block_2) false))))
    (:`then_2`
      (`self.K2_DestroyActor`))))

(fn `UserConstructionScript`)