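; Boss enemy that chases the player and deals damage through two attack hitboxes.
; Once StartTheAttack is set, Tick updates the player distance and uses CatchPlayer to either AI-move toward the player or stop, toggling FollowAnimation.
; Normal and hard trigger overlaps apply lighter or heavier damage to BP_MyCharacter, both playing a camera shake.
; BeginPlay stores the trigger and particle components in variables; nothing here sets the attack flags.
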(event `self.ReceiveBeginPlay`
  (set `self.damageParticle` (`self.DamageFX`))
  (set `self.normalTrigger` (`self.NormalAttack`))
  (set `self.hardTrigger` (`self.HardAttack`))
  (set `self.rockParticle` (`self.RockCrashFX`)))

(event `self.ReceiveTick`
  (params (DeltaSeconds :type "Float (single-precision)"))
  (if (`self.startTheAttack`)
    (`|ExecutionSequence`
      (:`then_0`
        (set `self.distanceToPlayer` (`self.GetDistanceTo` (`GameplayStatics.GetPlayerPawn` 0))))
      (:`then_1`
        (if (`self.catchPlayer`)
          (`|AIMoveTo` self (0.0 0.0 0.0) (`GameplayStatics.GetPlayerPawn` 0)
            (:`then`
              (`self.FollowAnimation` true)))
          (else
            (`MovementComponent.StopMovementImmediately` (`self.CharacterMovement`))
            (`self.FollowAnimation` false)))))))

(event `self.NormalAttack.OnComponentBeginOverlap`
  (params (OverlappedComponent :type "PrimitiveComponent Object Reference") (OtherActor :type "Actor Object Reference") (OtherComp :type "PrimitiveComponent Object Reference") (OtherBodyIndex :type Integer) (bFromSweep :type Boolean) (SweepResult :type "HitResult Structure (by ref)"))
  (bind _asbp_my_character (cast `/Game/Blueprints/Player/BP_MyCharacter` OtherActor))
  (`MyCharacter.NormalTakeDamage` _asbp_my_character 2.0)
  (`GameplayStatics.PlayWorldCameraShake` "/Game/Blueprints/CameraShakes/BP_TakeDamageCameraShake.BP_TakeDamageCameraShake_C" (`self.K2_GetActorLocation` (`GameplayStatics.GetPlayerPawn` 0)) 0.0 1000.0 :!label _label))

(event `self.HardAttack.OnComponentBeginOverlap`
  (params (OverlappedComponent :type "PrimitiveComponent Object Reference") (OtherActor :type "Actor Object Reference") (OtherComp :type "PrimitiveComponent Object Reference") (OtherBodyIndex :type Integer) (bFromSweep :type Boolean) (SweepResult :type "HitResult Structure (by ref)"))
  (bind _asbp_my_character (cast `/Game/Blueprints/Player/BP_MyCharacter` OtherActor))
  (`MyCharacter.HardTakeDamage` _asbp_my_character 4.0)
  (goto _label))

(fn `UserConstructionScript`)