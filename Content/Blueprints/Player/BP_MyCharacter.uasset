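; Player character Blueprint with camera-relative movement and three melee hit volumes: normal, hard and special.
; BeginPlay copies collision, effect and audio components into variables, and input is gated by cinematic, block, death and movement flags.
; Overlaps cast through fighter, shooter, magic and boss enemies to apply damage with camera shake.
; Normal and hard hits also play a cut sound and call TakePower, except on magic enemies.
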(event `self.ReceiveBeginPlay`
  (set `self.normalTrigger` (`self.NormalCollision`))
  (set `self.hardTrigger` (`self.HardCollision`))
  (set `self.damageParticle` (`self.DamageFX`))
  (set `self.hardDamageParticle` (`self.HardDamage`))
  (set `self.specialTrigger` (`self.SpecialCollision`))
  (set `self.SpecialEffect` (`self.SpecialFX`))
  (set `self.blockAudio` (`self.PlayerBlocks`)))

(event `self.ReceiveTick`
  (params (DeltaSeconds :type "Float (single-precision)"))
  ;[0.9659 1 0.9147] Para que el player mire en direccion a la camara, vamos a CharacterMovement y seteamos orient rotation to movement
  (set `self.movementDirection` (`KismetMathLibrary.MakeVector2D` (stale `InputAxis|Horizontal` AxisValue) (stale `InputAxis|Vertical` AxisValue))))

(event `InputAxis|Rotate`
  (params (AxisValue :type "Float (single-precision)"))
  ;[0.9659 1 0.9147] Para que el player mire en direccion a la camara, vamos a CharacterMovement y seteamos orient rotation to movement
  (if (not (`self.onCinematic`))
    (`self.AddControllerYawInput` AxisValue)))

(event `InputAxis|Vertical`
  (params (AxisValue :type "Float (single-precision)"))
  ;[0.9659 1 0.9147] Para que el player mire en direccion a la camara, vamos a CharacterMovement y seteamos orient rotation to movement
  (if (and (== (`self.canMove`) true) (== (`self.onBlockState`) false) (== (`self.playerIsDead`) false) (== (`self.onCinematic`) false))
    (`self.AddMovementInput` (`KismetMathLibrary.GetForwardVector` (`KismetMathLibrary.MakeRotator` 0.0 0.0 (.yaw (`self.GetControlRotation`)))) AxisValue)))

(event `InputAxis|Horizontal`
  (params (AxisValue :type "Float (single-precision)"))
  ;[0.9659 1 0.9147] Para que el player mire en direccion a la camara, vamos a CharacterMovement y seteamos orient rotation to movement
  (if (and (== (`self.canMove`) true) (== (`self.onBlockState`) false) (== (`self.playerIsDead`) false) (== (`self.onCinematic`) false))
    (`self.AddMovementInput` (`KismetMathLibrary.GetRightVector` (`KismetMathLibrary.MakeRotator` 0.0 0.0 (.yaw (`self.GetControlRotation`)))) AxisValue)))

(event `self.NormalCollision.OnComponentBeginOverlap`
  (params (OverlappedComponent :type "PrimitiveComponent Object Reference") (OtherActor :type "Actor Object Reference") (OtherComp :type "PrimitiveComponent Object Reference") (OtherBodyIndex :type Integer) (bFromSweep :type Boolean) (SweepResult :type "HitResult Structure (by ref)"))
  (bind _returnvalue (`self.K2_GetActorLocation`))
  (bind _asbp_my_fight_enemy (cast `/Game/Blueprints/Enemies/FightEnemy/BP_MyFightEnemy` OtherActor)
    (:`then`
      (`MyFightEnemy.TakeDamage` _asbp_my_fight_enemy 1.0)
      (`self.TakePower` 2.0)
      (`GameplayStatics.PlayWorldCameraShake` "/Game/Blueprints/CameraShakes/BP_NormalAttackCameraShake.BP_NormalAttackCameraShake_C" _returnvalue 0.0 1000.0 :!label _label))
    (:`CastFailed`
      (bind _asbp_shooter_enemy (cast `/Game/Blueprints/Enemies/ShooterEnemy/BP_ShooterEnemy` OtherActor)
        (:`then`
          (`ShooterEnemy.TakeDamage` _asbp_shooter_enemy 3.0)
          (`self.TakePower` 2.0)
          (goto _label))
        (:`CastFailed`
          (bind _asbp_magic_enemy (cast `/Game/Blueprints/Enemies/MagicEnemy/BP_MagicEnemy` OtherActor)
            (:`then`
              (`MagicEnemy.TakeDamage` _asbp_magic_enemy 2.0)
              (goto _label))
            (:`CastFailed`
              (bind _asbp_boss_enemy (cast `/Game/Blueprints/Enemies/Boss/BP_BossEnemy` OtherActor))
              (`BossEnemy.TakeDamage` _asbp_boss_enemy 2.0)
              (`self.TakePower` 2.0)
              (`GameplayStatics.PlayWorldCameraShake` "/Game/Blueprints/CameraShakes/BP_HardAttackCameraShake.BP_HardAttackCameraShake_C" _returnvalue 0.0 1000.0 :!label _label_2)))))))
  (`GameplayStatics.PlaySoundAtLocation` "/Game/Sounds/Player/PlayerCut.PlayerCut" _returnvalue (struct) 1.0 1.0 0.0 null null null))

(event `self.HardCollision.OnComponentBeginOverlap`
  (params (OverlappedComponent :type "PrimitiveComponent Object Reference") (OtherActor :type "Actor Object Reference") (OtherComp :type "PrimitiveComponent Object Reference") (OtherBodyIndex :type Integer) (bFromSweep :type Boolean) (SweepResult :type "HitResult Structure (by ref)"))
  (bind _asbp_my_fight_enemy (cast `/Game/Blueprints/Enemies/FightEnemy/BP_MyFightEnemy` OtherActor)
    (:`then`
      (`MyFightEnemy.TakeDamage` _asbp_my_fight_enemy 2.0)
      (`self.TakePower` 3.0)
      (goto _label_2))
    (:`CastFailed`
      (bind _asbp_shooter_enemy (cast `/Game/Blueprints/Enemies/ShooterEnemy/BP_ShooterEnemy` OtherActor)
        (:`then`
          (`ShooterEnemy.TakeDamage` _asbp_shooter_enemy 5.0)
          (`self.TakePower` 3.0)
          (goto _label_2))
        (:`CastFailed`
          (bind _asbp_magic_enemy (cast `/Game/Blueprints/Enemies/MagicEnemy/BP_MagicEnemy` OtherActor)
            (:`then`
              (`MagicEnemy.TakeDamage` _asbp_magic_enemy 3.0)
              (goto _label_2))
            (:`CastFailed`
              (bind _asbp_boss_enemy (cast `/Game/Blueprints/Enemies/Boss/BP_BossEnemy` OtherActor))
              (`BossEnemy.TakeDamage` _asbp_boss_enemy 3.0)
              (`self.TakePower` 3.0)
              (goto _label_2))))))))

(event `self.SpecialCollision.OnComponentBeginOverlap`
  (params (OverlappedComponent :type "PrimitiveComponent Object Reference") (OtherActor :type "Actor Object Reference") (OtherComp :type "PrimitiveComponent Object Reference") (OtherBodyIndex :type Integer) (bFromSweep :type Boolean) (SweepResult :type "HitResult Structure (by ref)"))
  (bind _asbp_my_fight_enemy (cast `/Game/Blueprints/Enemies/FightEnemy/BP_MyFightEnemy` OtherActor)
    (:`then`
      (`MyFightEnemy.TakeDamage` _asbp_my_fight_enemy 10.0))
    (:`CastFailed`
      (bind _asbp_shooter_enemy (cast `/Game/Blueprints/Enemies/ShooterEnemy/BP_ShooterEnemy` OtherActor)
        (:`then`
          (`ShooterEnemy.TakeDamage` _asbp_shooter_enemy 10.0))
        (:`CastFailed`
          (bind _asbp_magic_enemy (cast `/Game/Blueprints/Enemies/MagicEnemy/BP_MagicEnemy` OtherActor)
            (:`then`
              (`MagicEnemy.TakeDamage` _asbp_magic_enemy 5.0))
            (:`CastFailed`
              (bind _asbp_boss_enemy (cast `/Game/Blueprints/Enemies/Boss/BP_BossEnemy` OtherActor))
              (`BossEnemy.TakeDamage` _asbp_boss_enemy 5.0)))))))
  (`GameplayStatics.PlayWorldCameraShake` "/Game/Blueprints/CameraShakes/BP_SpecialAttackCameraShake.BP_SpecialAttackCameraShake_C" (`self.K2_GetActorLocation`) 0.0 1000.0))

(fn `UserConstructionScript`)